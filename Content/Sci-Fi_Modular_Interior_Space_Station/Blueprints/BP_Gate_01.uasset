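; BP_Gate_01 is a sci-fi gate that slides open when a Character enters its Box trigger.
; The Move timeline drives three mesh panels, one up and two sideways, by setting their relative transforms.
; Any actor leaving the separate Box1 volume reverses the timeline to close it.
; Box also toggles player 0's input on the gate, though the graph handles no input events.
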(event OnComponentEndOverlap(Box1)
  (params (OverlappedComponent :type Primitive%20Component%20Object%20Reference) (OtherActor :type Actor%20Object%20Reference) (OtherComp :type Primitive%20Component%20Object%20Reference) (OtherBodyIndex :type Integer))
  (bind (_direction _moveup _moveright _moveleft) (Timeline|Move Reverse)
    (:Update
      (Transformation|SetRelativeTransform (Variables|Default|GetSM_Gate_01_Gate_01_Up) (Math|Transform|MakeTransform _moveup) false false)
      (Transformation|SetRelativeTransform (Variables|Default|GetSM_Gate_01_Gate_01_Side) (Math|Transform|MakeTransform _moveleft) false false)
      (Transformation|SetRelativeTransform (Variables|Default|GetSM_Gate_01_Gate_01_Side2) (Math|Transform|MakeTransform _moveright "0,180.000000, 0") false false))))

(event OnComponentBeginOverlap(Box)
  (params (OverlappedComponent :type Primitive%20Component%20Object%20Reference) (OtherActor :type Actor%20Object%20Reference) (OtherComp :type Primitive%20Component%20Object%20Reference) (OtherBodyIndex :type Integer) (bFromSweep :type Boolean) (SweepResult :type Hit%20Result%20Structure%20%28by%20ref%29))
  (Utilities|Casting|CastToCharacter OtherActor)
  (Input|EnableInput (Game|GetPlayerController 0))
  (bind (_direction _moveup _moveright _moveleft) (Timeline|Move Play)
    (:Update
      (Transformation|SetRelativeTransform (Variables|Default|GetSM_Gate_01_Gate_01_Up) (Math|Transform|MakeTransform _moveup) false false)
      (Transformation|SetRelativeTransform (Variables|Default|GetSM_Gate_01_Gate_01_Side) (Math|Transform|MakeTransform _moveleft) false false)
      (Transformation|SetRelativeTransform (Variables|Default|GetSM_Gate_01_Gate_01_Side2) (Math|Transform|MakeTransform _moveright "0,180.000000, 0") false false))))

(event OnComponentEndOverlap(Box)
  (params (OverlappedComponent :type Primitive%20Component%20Object%20Reference) (OtherActor :type Actor%20Object%20Reference) (OtherComp :type Primitive%20Component%20Object%20Reference) (OtherBodyIndex :type Integer))
  (Utilities|Casting|CastToCharacter OtherActor)
  (Input|DisableInput (Game|GetPlayerController 0)))

(fn ConstructionScript)