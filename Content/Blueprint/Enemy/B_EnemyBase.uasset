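; B_EnemyBase is the base enemy actor, providing normalized health and spatial queries for allies and free positions.
; Each tick it destroys itself at zero health or caps health at 1, and calls an unfinished RollWheel.
; Sphere traces gather nearby actors or B_EnemyBase allies.
; FindFreePosition samples random reachable navmesh points for an ally-free spot within a retry limit, but re-rolls the point it returns rather than keeping the tested one.
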(event EventBeginPlay)

(event Collision|EventActorBeginOverlap
  (params (OtherActor :type Actor%20Object%20Reference)))

(event EventTick
  (params (DeltaSeconds :type Float%20%28single-precision%29))
  (CallFunction|CheckHealth)
  (CallFunction|RollWheel DeltaSeconds))

(fn ConstructionScript)

(fn GetHealth
  (return (Variables|Default|GetHealth)))

(fn Damage
  (params (Ammount :type Float%20%28double-precision%29))
  (Variables|Default|SetHealth (- (Variables|Default|GetHealth) Ammount)))

(fn CheckHealth
  (if (<= (Variables|Default|GetHealth) 0.0)
    (Actor|DestroyActor)
    (return)
    (elif (> (Variables|Default|GetHealth) 1.0)
      (Variables|Default|SetHealth 1.0)
      (return))))

(fn RollWheel
  (params (DeltaTime :type Float%20%28double-precision%29))
  ;[1 1 1] Apply Rotation
  (if (Utilities|IsValid 0)
    _))

(fn GetLocalAllies
  (bind _returnvalue (Transformation|GetActorLocation))
  (bind _outhits (Collision|MultiSphereTraceForObjects _returnvalue _returnvalue (LocalVariables|GetSearchDistance) (LocalVariables|GetTraceType) false 0 "None"))
  (for _array_element _outhits
    (Utilities|Array|Add (LocalVariables|GetReturnArray) (.HitActor (Collision|BreakHitResult _array_element))))
  (return (LocalVariables|GetReturnArray)))

(fn GetAlliesNearPoint
  (params (Position :type Vector) (Range :type Float%20%28double-precision%29))
  (bind _outhits (Collision|MultiSphereTraceForObjects Position Position Range (LocalVariables|GetTargetType) false 0 "None"))
  (for _array_element _outhits
    (bind _asb_enemy_base (Utilities|Casting|CastToB_EnemyBase (.HitActor (Collision|BreakHitResult _array_element))))
    (Utilities|Array|Add (LocalVariables|GetResultArray) _asb_enemy_base))
  (return (LocalVariables|GetResultArray)))

(fn FindFreePosition
  (params (Range :type Float%20%28double-precision%29))
  (bind _returnvalue (Transformation|GetActorLocation))
  (bind _randomlocation (AI|Navigation|GetRandomReachablePointinRadius _returnvalue Range 0 0))
  ;[1 1 1] Default return position is pos of actor
  (LocalVariables|SetResultPoint (.RandomLocation (AI|Navigation|GetRandomReachablePointinRadius _returnvalue Range 0 0)))
  ;[1 1 1] Only check so many times
  (while (< (LocalVariables|GetCheckCount) (LocalVariables|GetCheckLimit))
    ;[1 1 1] Is allies near point? If so go +1 to loop end
    (bind _actors (CallFunction|GetAlliesNearPoint _randomlocation 3e+02))
    (if (== (Utilities|Array|Length _actors) 0)
      (LocalVariables|SetResultPoint _randomlocation)
      (LocalVariables|SetCheckCount (LocalVariables|GetCheckLimit))
      (else
        (LocalVariables|SetCheckCount (+ (LocalVariables|GetCheckCount) 1)))))
  (return (LocalVariables|GetResultPoint)))