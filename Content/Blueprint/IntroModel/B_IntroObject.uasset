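; Intro scene actor that shows a slowly spinning skeletal mesh over dark ambience before the game starts.
; On BeginPlay it makes itself the player's view target and plays a 2D ambient sound, while Tick steadily yaws the mesh.
; Pressing Enter opens the Station level and destroys the actor.
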(event EventBeginPlay
  (CallFunction|Init))

(event Collision|EventActorBeginOverlap
  (params (OtherActor :type Actor%20Object%20Reference)))

(event EventTick
  (params (DeltaSeconds :type Float%20%28single-precision%29))
  (CallFunction|SpinHead DeltaSeconds))

(event Input|KeyboardEvents|Enter
  (params (Key :type Key%20Structure))
  (:Pressed
    (Game|OpenLevel(byObjectReference) "/Game/Level/L_Station.L_Station")
    (Actor|DestroyActor)))

(fn ConstructionScript)

(fn SpinHead
  (params (DeltaTime :type Float%20%28double-precision%29))
  (Transformation|AddRelativeRotation (Variables|Default|GetSkeletalMesh) (Math|Rotator|MakeRotator 0.0 0.0 (* DeltaTime 4e+01)) false false))

(fn Init
  (Game|Player|SetViewTargetwithBlend (Game|GetPlayerController 0) self 0.0 "VTBlend_Linear" 0.0 false)
  (Audio|PlaySound2D "/Game/Sounds/Music/SC_DarkAmbience.SC_DarkAmbience" 1.0 1.0 0.0 0 0))