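; BlockerBox is an actor that acts as a toggleable collision blocker through its Collider component.
; An Active flag sets the Collider's response on all channels to Block when true and Ignore when false.
; The response is applied on BeginPlay and again whenever SetActive changes the flag.
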(event EventBeginPlay
  (CallFunction|RefreshCollisionProperty))

(event Collision|EventActorBeginOverlap
  (params (OtherActor :type Actor%20Object%20Reference)))

(event EventTick
  (params (DeltaSeconds :type Float%20%28single-precision%29)))

(fn ConstructionScript)

(fn RefreshCollisionProperty
  (if (Variables|Default|GetActive)
    (Collision|SetCollisionResponsetoAllChannels (Variables|Default|GetCollider) "ECR_Block")
    (else
      (Collision|SetCollisionResponsetoAllChannels (Variables|Default|GetCollider) "ECR_Ignore"))))

(fn SetActive
  (params (NewValue :type Boolean))
  (Variables|Default|SetActive NewValue)
  (CallFunction|RefreshCollisionProperty))