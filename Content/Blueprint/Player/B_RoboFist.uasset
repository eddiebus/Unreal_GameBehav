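; B_RoboFist is a robotic fist actor that punches its Knuckle component forward and pulls it back.
; Fire sets a velocity, which decays by PullBackSpeed each Tick and drives a distance clamped between zero and MaxDistance, adjustable through SetPunchDistance.
; That distance sets the knuckle's relative location along local forward, without sweep.
; Overlap only prints a debug string, and Init and PushPhysicProp are empty stubs.
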(event EventBeginPlay
  (CallFunction|Init))

(event Collision|EventActorBeginOverlap
  (params (OtherActor :type Actor%20Object%20Reference))
  (Development|PrintString "Knuckle Hit"))

(event EventTick
  (params (DeltaSeconds :type Float%20%28single-precision%29))
  (CallFunction|UpdateDistance DeltaSeconds)
  (CallFunction|SetKnucklePosition))

(fn ConstructionScript)

(fn Init)

(fn SetPunchDistance
  (params (NewValue :type Float%20%28double-precision%29))
  (Variables|Default|SetMaxDistance NewValue)
  (return))

(fn SetKnucklePosition
  (Transformation|SetRelativeLocation (Variables|Default|GetKnuckle) (* (Math|Vector|GetForwardVector "0, 0, 0") (* (Variables|Default|GetCurrentDistance) 1e+01)) false false))

(fn UpdateDistance
  (params (timeDelta :type Float%20%28double-precision%29))
  (bind _output_get (LocalVariables|SetcurrentDeltaTime timeDelta))
  (CallFunction|UpdateVelocity _output_get)
  (Variables|Default|SetCurrentDistance (+ (Variables|Default|GetCurrentDistance) (Variables|Default|GetVelocity)))
  (if (> (Variables|Default|GetCurrentDistance) (Variables|Default|GetMaxDistance))
    (Variables|Default|SetCurrentDistance (Variables|Default|GetMaxDistance)))
  (Variables|Default|SetCurrentDistance (- (Variables|Default|GetCurrentDistance) (LocalVariables|GetcurrentDeltaTime)))
  (if (< (Variables|Default|GetCurrentDistance) 0.0)
    (Variables|Default|SetCurrentDistance 0.0)))

(fn Fire
  (params (PunchSpeed :type Float%20%28double-precision%29))
  (Variables|Default|SetVelocity PunchSpeed))

(fn UpdateVelocity
  (params (DeltaTime :type Float%20%28double-precision%29))
  (LocalVariables|SetcurrentDeltaTime DeltaTime)
  (Variables|Default|SetVelocity (- (Variables|Default|GetVelocity) (* (Variables|Default|Get_PullBackSpeed) (LocalVariables|GetcurrentDeltaTime))))
  (return))

(fn PushPhysicProp
  (params (OtherObj :type Actor%20Object%20Reference)))