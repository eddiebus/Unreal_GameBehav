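; B_PlayerRobo is the first-person-style player robot, with mouse look, WASD movement, two fist weapons, health and score.
; Tick polls raw input to move along capsule axes, yaw the capsule, and pitch the camera and both fists together.
; Left and right mouse buttons fire the matching B_RoboFist child actor.
; Overlapping Bullets subtract health and are destroyed; movement, look and firing stop at zero health.
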(event EventBeginPlay
  (CallFunction|Init))

(event Collision|EventActorBeginOverlap
  (params (OtherActor :type Actor%20Object%20Reference))
  (CallFunction|TakeDamagefromBullet OtherActor))

(event EventTick
  (params (DeltaSeconds :type Float%20%28single-precision%29))
  (CallFunction|Move)
  (CallFunction|Look))

(event Input|MouseEvents|LeftMouseButton
  (params (Key :type Key%20Structure))
  (:Pressed
    (if (> (Variables|Default|GetPlayer_HP) 0.0)
      (bind _asb_robo_fist (Utilities|Casting|CastToB_RoboFist (Variables|/Script/Engine.ChildActorComponent|GetChildActor (Variables|Default|GetLeftKnuckle))))
      (Default|Fire _asb_robo_fist 1e+01))))

(event Input|MouseEvents|RightMouseButton
  (params (Key :type Key%20Structure))
  (:Pressed
    (if (> (Variables|Default|GetPlayer_HP) 0.0)
      (bind _asb_robo_fist (Utilities|Casting|CastToB_RoboFist (Variables|/Script/Engine.ChildActorComponent|GetChildActor (Variables|Default|GetRightFist))))
      (Default|Fire _asb_robo_fist 1e+01))))

(fn ConstructionScript)

(fn Init
  (Game|Player|SetViewTargetwithBlend (Game|GetPlayerController 0) self 0.0 "VTBlend_Linear" 0.0 false))

(fn Look
  (bind _returnvalue (Game|GetPlayerController 0))
  (bind (_deltax _deltay) (Class|PlayerController|GetInputMouseDelta _returnvalue))
  (if (> (Variables|Default|GetPlayer_HP) 0.0)
    (LocalVariables|SetLookDelta (Math|Vector|MakeVector _deltax _deltay 0.0))
    (Transformation|AddWorldRotation (Variables|Collision|GetCapsuleComponent) (Math|Rotator|MakeRotator 0.0 0.0 (.x (LocalVariables|GetLookDelta))) false false)
    (Pawn|Input|AddControllerYawInput 0.0)
    (Transformation|AddLocalRotation (Variables|Default|GetCamera) (Math|Rotator|MakeRotator 0.0 (.y (LocalVariables|GetLookDelta)) 0.0) false false)
    (CallFunction|RotateFistYDelta (.y (LocalVariables|GetLookDelta)))
    (Class|PrimitiveComponent|SetPhysicsMaxAngularVelocityinDegrees (Variables|Collision|GetCapsuleComponent) 0.0 false "None")))

(fn Move
  ;[1 1 1] Forward Back (W/S)
  ;;[1 1 1] Forward
  (if (> (Variables|Default|GetPlayer_HP) 0.0)
    (if (Game|Player|IsInputKeyDown (Game|GetPlayerController 0) "W")
      (bind _returnvector (CallFunction|GetForwardMoveVector))
      (Pawn|Input|AddMovementInput _returnvector 1.0 false))
    ;;[1 1 1] Back
    (if (Game|Player|IsInputKeyDown (Game|GetPlayerController 0) "S")
      (bind _returnvector_2 (CallFunction|GetForwardMoveVector))
      (Pawn|Input|AddMovementInput (* _returnvector_2 -1.0) 1.0 false))
    ;[1 1 1] Strafe Movement (A/D
    ;;[1 1 1] Right Strafe
    (bind _returnvector_3 (CallFunction|GetForwardMoveVector))
    (LocalVariables|SetStrafeVector (Math|Vector|RotateVector _returnvector_3 "0,90.000000, 0"))
    (if (Game|Player|IsInputKeyDown (Game|GetPlayerController 0) "D")
      (Pawn|Input|AddMovementInput (LocalVariables|GetStrafeVector) 1.0 false))
    ;;[1 1 1] Left Strafe
    (if (Game|Player|IsInputKeyDown (Game|GetPlayerController 0) "A")
      (Pawn|Input|AddMovementInput (* (LocalVariables|GetStrafeVector) -1.0) 1.0 false))))

(fn GetForwardMoveVector
  (return (* (Math|Vector|GetForwardVector (Variables|Collision|GetCapsuleComponent)) (Variables|Default|GetWalkSpeed))))

(fn RotateFistYDelta
  (params (yDelta%20 :type Float%20%28double-precision%29))
  (Transformation|AddRelativeRotation (Variables|Default|GetRightFist) (Math|Rotator|MakeRotator 0.0 yDelta%20 0.0) false false)
  (Transformation|AddRelativeRotation (Variables|Default|GetLeftKnuckle) (Math|Rotator|MakeRotator 0.0 yDelta%20 0.0) false false))

(fn TakeDamagefromBullet
  (params (OtherObj :type Object%20Object%20Reference))
  (bind _asbullet (Utilities|Casting|CastToBullet OtherObj))
  (bind _damage (Default|GetDamage _asbullet))
  (Variables|Default|SetPlayer_HP (- (Variables|Default|GetPlayer_HP) _damage))
  (Actor|DestroyActor _asbullet)
  (return))

(fn AddScore
  (params (Points :type Integer))
  (Variables|Default|SetScore (+ (Variables|Default|GetScore) Points)))

(fn GetScore
  (return (Variables|Default|GetScore)))

(fn Damage
  (params (DamageToTake :type Float%20%28double-precision%29))
  (Variables|Default|SetPlayer_HP (- (Variables|Default|GetPlayer_HP) DamageToTake))
  (return))

(fn GetHealth
  (return (Variables|Default|GetPlayer_HP)))