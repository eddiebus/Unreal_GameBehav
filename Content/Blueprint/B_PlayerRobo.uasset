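; Player robot pawn that walks, looks around in first-person style and fires two fist child actors.
; It takes the view target on BeginPlay, then each tick polls WASD for movement input along the capsule's forward and strafe vectors.
; Mouse delta yaws the capsule and pitches the camera and both fists together, without clamping.
; Left and right clicks call Fire on the matching B_RoboFist child actor.
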(event EventBeginPlay
  (CallFunction|Init))

(event Collision|EventActorBeginOverlap
  (params (OtherActor :type Actor%20Object%20Reference)))

(event EventTick
  (params (DeltaSeconds :type Float%20%28single-precision%29))
  (CallFunction|Move)
  (CallFunction|Look))

(event Input|MouseEvents|LeftMouseButton
  (params (Key :type Key%20Structure :default "None"))
  (:Pressed
    (bind _asb_robo_fist (Utilities|Casting|CastToB_RoboFist (Variables|/Script/Engine.ChildActorComponent|GetChildActor (Variables|Default|GetLeftKnuckle))))
    (Default|Fire _asb_robo_fist 1e+01)))

(event Input|MouseEvents|RightMouseButton
  (params (Key :type Key%20Structure :default "None"))
  (:Pressed
    (bind _asb_robo_fist (Utilities|Casting|CastToB_RoboFist (Variables|/Script/Engine.ChildActorComponent|GetChildActor (Variables|Default|GetRightFist))))
    (Default|Fire _asb_robo_fist 1e+01)))

(fn ConstructionScript)

(fn Init
  (Game|Player|SetViewTargetwithBlend (Game|GetPlayerController 0) self 0.0 "VTBlend_Linear" 0.0 false))

(fn Look
  (bind _returnvalue (Game|GetPlayerController 0))
  (bind (_deltax _deltay) (Class|PlayerController|GetInputMouseDelta _returnvalue))
  (LocalVariables|SetLookDelta (Math|Vector|MakeVector _deltax _deltay 0.0))
  (Transformation|AddWorldRotation (Variables|Collision|GetCapsuleComponent) (Math|Rotator|MakeRotator 0.0 0.0 (.x (LocalVariables|GetLookDelta))) false false)
  (Pawn|Input|AddControllerYawInput 0.0)
  (Transformation|AddLocalRotation (Variables|Default|GetCamera) (Math|Rotator|MakeRotator 0.0 (.y (LocalVariables|GetLookDelta)) 0.0) false false)
  (CallFunction|RotateFistYDelta (.y (LocalVariables|GetLookDelta)))
  (Class|PrimitiveComponent|SetPhysicsMaxAngularVelocityinDegrees (Variables|Collision|GetCapsuleComponent) 0.0 false "None"))

(fn Move
  ;[1 1 1] Forward Back (W/S)
  ;;[1 1 1] Forward
  (if (Game|Player|IsInputKeyDown (Game|GetPlayerController 0) "W")
    (bind _returnvector (CallFunction|GetForwardMoveVector))
    (Pawn|Input|AddMovementInput _returnvector 1.0 false))
  ;;[1 1 1] Back
  (if (Game|Player|IsInputKeyDown (Game|GetPlayerController 0) "S")
    (bind _returnvector_2 (CallFunction|GetForwardMoveVector))
    (Pawn|Input|AddMovementInput (* _returnvector_2 -1.0) 1.0 false))
  ;[1 1 1] Strafe Movement (A/D
  ;;[1 1 1] Right Strafe
  (bind _returnvector_3 (CallFunction|GetForwardMoveVector))
  (LocalVariables|SetStrafeVector (Math|Vector|RotateVector _returnvector_3 "0,90.000000, 0"))
  (if (Game|Player|IsInputKeyDown (Game|GetPlayerController 0) "D")
    (Pawn|Input|AddMovementInput (LocalVariables|GetStrafeVector) 1.0 false))
  ;;[1 1 1] Left Strafe
  (if (Game|Player|IsInputKeyDown (Game|GetPlayerController 0) "A")
    (Pawn|Input|AddMovementInput (* (LocalVariables|GetStrafeVector) -1.0) 1.0 false)))

(fn GetForwardMoveVector
  (return (* (Math|Vector|GetForwardVector (Variables|Collision|GetCapsuleComponent)) (Variables|Default|GetWalkSpeed))))

(fn RotateFistYDelta
  (params (yDelta%20 :type Float%20%28double-precision%29))
  (Transformation|AddRelativeRotation (Variables|Default|GetRightFist) (Math|Rotator|MakeRotator 0.0 yDelta%20 0.0) false false)
  (Transformation|AddRelativeRotation (Variables|Default|GetLeftKnuckle) (Math|Rotator|MakeRotator 0.0 yDelta%20 0.0) false false))