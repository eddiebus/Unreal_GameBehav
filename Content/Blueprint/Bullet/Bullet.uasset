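; Bullet is a projectile actor that travels along a set direction and destroys itself when its lifetime runs out.
; Each Tick, Move overwrites the StaticMesh's physics linear velocity with direction times scaled speed and delta time, so velocity varies with frame rate.
; Age counts the lifetime down by delta time and destroys the actor at zero.
; Setter functions supply speed, direction and lifetime, while Init is empty.
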(event EventBeginPlay)

(event Collision|EventActorBeginOverlap
  (params (OtherActor :type Actor%20Object%20Reference)))

(event EventTick
  (params (DeltaSeconds :type Float%20%28single-precision%29))
  (CallFunction|Move DeltaSeconds)
  (CallFunction|Age DeltaSeconds))

(fn ConstructionScript)

(fn Move
  (params (DeltaTime :type Float%20%28double-precision%29))
  (LocalVariables|SetTime DeltaTime)
  (bind _output_get (LocalVariables|SetMoveVector (* (Variables|Default|GetDirection) (* (* (Variables|Default|GetSpeed) 1e+04) (LocalVariables|GetTime)))))
  (Physics|SetPhysicsLinearVelocity (Variables|Default|GetStaticMesh) _output_get false "None"))

(fn SetSpeed
  (params (NewSpeed :type Float%20%28double-precision%29))
  (Variables|Default|SetSpeed NewSpeed)
  (return))

(fn SetDirection
  (params (SetDirection :type Vector))
  (Variables|Default|SetDirection SetDirection)
  (return))

(fn SetBulletTime
  (params (NewTime :type Float%20%28double-precision%29))
  (Variables|Default|SetLifeTime NewTime)
  (return))

(fn Age
  (params (DeltaTime :type Float%20%28double-precision%29))
  ;[1 1 1] Age Bullet
  (Variables|Default|SetLifeTime (- (Variables|Default|GetLifeTime) DeltaTime))
  ;[1 1 1] Delete Self if Aged
  (if (<= (Variables|Default|GetLifeTime) 0.0)
    (Actor|DestroyActor)))

(fn Init)