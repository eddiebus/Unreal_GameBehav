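; B_PlayArea is a trigger actor that starts a combat encounter when the player robot (B_PlayerRobo) overlaps it.
; On the first overlap it activates its referenced enemy robot spawners and blocker boxes, then starts looping fight music.
; An Active flag keeps the encounter from triggering again, and nothing in this Blueprint resets it or ends the fight.
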(event EventBeginPlay)

(event Collision|EventActorBeginOverlap
  (params (OtherActor :type Actor%20Object%20Reference))
  (Utilities|Casting|CastToB_PlayerRobo OtherActor)
  (CallFunction|TriggerPlayArea))

(event EventTick
  (params (DeltaSeconds :type Float%20%28single-precision%29)))

(fn ConstructionScript)

(fn TriggerPlayArea
  (if (not (Variables|Default|GetActive))
    (CallFunction|ActivateSpawners)
    (CallFunction|ActivateBlockers)
    (Audio|PlaySound2D "/Game/Sounds/Music/SC_FightMusicLoop.SC_FightMusicLoop" 1.0 1.0 0.0 0 0)
    (Variables|Default|SetActive true)))

(fn ActivateSpawners
  (for _array_element (Variables|Default|GetEnemySpawner)
    (bind _asb_enemy_robo_spawner (Utilities|Casting|CastToB_EnemyRoboSpawner _array_element))
    (Default|SetActive _asb_enemy_robo_spawner true))
  (return))

(fn ActivateBlockers
  (for _array_element (Variables|Default|GetBlockerPoints)
    (bind _asblocker_box (Utilities|Casting|CastToBlockerBox _array_element))
    (Default|SetActive _asblocker_box true))
  (return))